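; BP_Enemy is an enemy actor that damages the player on contact or awards points when shot.
; Overlapping BP_Player calls its ProcessHit, while a hit from BP_Projectile increments the player's combo and score and adds a new combo widget to the viewport.
; Tick checks whether the enemy has fallen behind the player along X, triggering EnemyMissed to reset the combo.
; All three outcomes destroy the enemy.
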(event OnComponentBeginOverlap(EnemyCollision)
  (params (OverlappedComponent :type Primitive%20Component%20Object%20Reference) (OtherActor :type Actor%20Object%20Reference) (OtherComp :type Primitive%20Component%20Object%20Reference) (OtherBodyIndex :type Integer) (bFromSweep :type Boolean) (SweepResult :type Hit%20Result%20Structure%20%28by%20ref%29))
  (bind _asbp_player (Utilities|Casting|CastToBP_Player OtherActor))
  (Default|ProcessHit _asbp_player 25.0)
  (Actor|DestroyActor))

(event OnComponentHit(EnemyCollision)
  (params (HitComponent :type Primitive%20Component%20Object%20Reference) (OtherActor :type Actor%20Object%20Reference) (OtherComp :type Primitive%20Component%20Object%20Reference) (NormalImpulse :type Vector :default "0, 0, 0") (Hit :type Hit%20Result%20Structure%20%28by%20ref%29))
  (Utilities|Casting|CastToBP_Projectile OtherActor)
  (bind _asbp_player (Utilities|Casting|CastToBP_Player (Game|Player|GetPlayerPawn 0)))
  (Variables|/Game/InfiniteMatrix/Blueprints/BP_Player.BP_Player_C|SetCombo _asbp_player (+ (Variables|/Game/InfiniteMatrix/Blueprints/BP_Player.BP_Player_C|GetCombo _asbp_player) 1))
  (bind _returnvalue (UserInterface|CreateWidget "/Game/InfiniteMatrix/UI/WBP_Combo.WBP_Combo_C"))
  (UserInterface|Viewport|AddtoViewport _returnvalue 0)
  (Variables|/Game/InfiniteMatrix/Blueprints/BP_Player.BP_Player_C|SetScore _asbp_player (+ (Variables|/Game/InfiniteMatrix/Blueprints/BP_Player.BP_Player_C|GetScore _asbp_player) 1))
  (Actor|DestroyActor))

(event Custom|EnemyMissed
  (Development|PrintString "Enemy Missed")
  (bind _asbp_player (Utilities|Casting|CastToBP_Player (Game|Player|GetPlayerPawn 0)))
  (Variables|/Game/InfiniteMatrix/Blueprints/BP_Player.BP_Player_C|SetCombo _asbp_player 0)
  (Actor|DestroyActor))

(event EventBeginPlay)

(event Collision|EventActorBeginOverlap
  (params (OtherActor :type Actor%20Object%20Reference)))

(event EventTick
  (params (DeltaSeconds :type Float%20%28single-precision%29))
  (if (< (.x (Transformation|GetActorLocation)) (- (.x (Transformation|GetActorLocation (Game|Player|GetPlayerPawn 0))) 2e+02))
    (CallFunction|EnemyMissed)))

(fn ConstructionScript)